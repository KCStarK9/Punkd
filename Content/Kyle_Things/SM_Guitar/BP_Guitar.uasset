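; BP_Guitar is a guitar prop actor assembled from separate body, neck, pickup and peg components.
; On BeginPlay it sets the first material slot of each component from the Body, Neck, Pickups and Pegs values, so each part gets its own material.
; The construction script is empty, so these materials are applied only at runtime, and the overlap and tick events do nothing.
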(event `self.ReceiveBeginPlay`
  (`PrimitiveComponent.SetMaterial` (`self.Guitar_Body`) 0 (`self.Body`))
  (`PrimitiveComponent.SetMaterial` (`self.Guitar_Neck`) 0 (`self.Neck`))
  (`PrimitiveComponent.SetMaterial` (`self.Guitar_Pickup`) 0 (`self.Pickups`))
  (`PrimitiveComponent.SetMaterial` (`self.Guitar_Pegs`) 0 (`self.Pegs`)))

(fn `UserConstructionScript`)