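; BP_Punk is an AI character that moves toward the player pawn five seconds after spawning, with physics-driven body motion.
; On BeginPlay it applies Physical Animation to the mesh from a configured bone down and simulates physics on the bodies below it, blending animation with physical reaction.
; It binds to the CHOOSING event on BP_PunkdController, which disables the punk's movement when fired.
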(event `Freeze`
  (`CharacterMovementComponent.DisableMovement` (`self.CharacterMovement`)))

(event `self.ReceiveBeginPlay`
  (bind _physicalanimation (`self.PhysicalAnimation`))
  (bind _bone (`self.Bone`))
  (`PhysicalAnimationComponent.SetSkeletalMeshComponent` _physicalanimation (`self.Mesh`))
  (`PhysicalAnimationComponent.ApplyPhysicalAnimationSettingsBelow` _physicalanimation _bone (make `PhysicalAnimationData` true 1000.0 100.0 1000.0 100.0 100.0 100.0) true)
  (`SkeletalMeshComponent.SetAllBodiesBelowSimulatePhysics` (`self.Mesh`) _bone true false)
  (bind _asbp_punkd_controller (cast `/Game/Casey_Stuff/BP_PunkdController` (`GameplayStatics.GetPlayerController` 0)))
  (bind _output_get (set `self.MainController` _asbp_punkd_controller))
  (add `/Game/Casey_Stuff/BP_PunkdController.CHOOSING` _output_get (delegate `Freeze`))
  (`KismetSystemLibrary.Delay` 5.0)
  (`|AIMoveTo` self (0.0 0.0 0.0) (`GameplayStatics.GetPlayerPawn` 0)))

(fn `UserConstructionScript`)