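; Player pawn that moves along world X and freezes while a choice is pending.
; On BeginPlay it applies physical animation below a root bone and simulates the bodies under it for physics-driven motion.
; It binds to BP_PunkdController's CHOOSING and CHOICEMADE events to disable movement, then restore walking.
; Look events toggle between front and back cameras.
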(event `UnFreeze`
  (`CharacterMovementComponent.SetMovementMode` (`self.CharacterMovement`) "MOVE_Walking" 0))

(event `self.ReceiveBeginPlay`
  (bind _bone (`self.Bone`))
  (bind _physicalanimation (`self.PhysicalAnimation`))
  (`PhysicalAnimationComponent.SetSkeletalMeshComponent` _physicalanimation (`self.Mesh`))
  (`PhysicalAnimationComponent.ApplyPhysicalAnimationSettingsBelow` _physicalanimation _bone (make `PhysicalAnimationData` true 1000.0 100.0 1000.0 100.0 100.0 100.0) true)
  (`SkeletalMeshComponent.SetAllBodiesBelowSimulatePhysics` (`self.Mesh`) _bone true false)
  (bind _asbp_punkd_controller (cast `/Game/Casey_Stuff/BP_PunkdController` (`GameplayStatics.GetPlayerController` 0)))
  (add `/Game/Casey_Stuff/BP_PunkdController.CHOOSING` _asbp_punkd_controller (delegate `Freeze`))
  (add `/Game/Casey_Stuff/BP_PunkdController.CHOICEMADE` _asbp_punkd_controller (delegate `UnFreeze`)))

(event `LookBehind`
  (`ActorComponent.Activate` (`self.BackCamera`) false)
  (`ActorComponent.Deactivate` (`self.FrontCamera`)))

(event `LookAhead`
  (`ActorComponent.Activate` (`self.FrontCamera`) false)
  (`ActorComponent.Deactivate` (`self.BackCamera`)))

(event `Freeze`
  (`CharacterMovementComponent.DisableMovement` (`self.CharacterMovement`)))

(event `Move`
  (`self.AddMovementInput` (1.0 0.0 0.0)))

(fn `UserConstructionScript`)