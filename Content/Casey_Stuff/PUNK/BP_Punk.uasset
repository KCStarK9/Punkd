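; BP_Punk is a punk character that calls PUNKing on BP_PunkdController when the player pawn enters its PUNKingradius.
; At BeginPlay it applies physical animation, simulating physics on bodies below a chosen bone.
; Controller CHOOSING and CHOICEMADE events freeze and restore its walking movement.
; A Delay loop started from Tick repeatedly gives a random spike a random neon material for a flickering look.
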(event `Freeze`
  (`CharacterMovementComponent.DisableMovement` (`self.CharacterMovement`)))

(event `self.ReceiveBeginPlay`
  (bind _physicalanimation (`self.PhysicalAnimation`))
  (bind _bone (`self.Bone`))
  (`PhysicalAnimationComponent.SetSkeletalMeshComponent` _physicalanimation (`self.Mesh`))
  (`PhysicalAnimationComponent.ApplyPhysicalAnimationSettingsBelow` _physicalanimation _bone (make `PhysicalAnimationData` true 1000.0 100.0 1000.0 100.0 100.0 100.0) true)
  (`SkeletalMeshComponent.SetAllBodiesBelowSimulatePhysics` (`self.Mesh`) _bone true false)
  (bind _asbp_punkd_controller (cast `/Game/Casey_Stuff/BP_PunkdController` (`GameplayStatics.GetPlayerController` 0)))
  (bind _output_get (set `self.MainController` _asbp_punkd_controller))
  (add `/Game/Casey_Stuff/BP_PunkdController.CHOOSING` _output_get (delegate `Freeze`))
  (add `/Game/Casey_Stuff/BP_PunkdController.CHOICEMADE` _output_get (delegate `Unfreeze`)))

(event `Unfreeze`
  (`CharacterMovementComponent.SetMovementMode` (`self.CharacterMovement`) "MOVE_Walking" 0))

(event `self.ReceiveTick`
  (params (DeltaSeconds :type "Float (single-precision)"))
  (`KismetSystemLibrary.Delay` 0.1 :!label _label)
  (`PrimitiveComponent.SetMaterial` (`KismetArrayLibrary.Array_Random` (`|MakeArray` (`self.Spike_1`) (`self.Spike_2`) (`self.Spike_3`) (`self.Spike_4`) (`self.Spike_5`))) 0 (`KismetArrayLibrary.Array_Random` (`|MakeArray` "/Game/Morgan/Neon.Neon" "/Game/Morgan/Neon_Green.Neon_Green" "/Game/Morgan/Neon_Pink.Neon_Pink" "/Game/Morgan/Neon_Purple.Neon_Purple" "/Game/Morgan/Neon_Red.Neon_Red" :!type "MaterialInterface Object Reference")))
  (goto _label))

(event `self.PUNKingradius.OnComponentBeginOverlap`
  (params (OverlappedComponent :type "PrimitiveComponent Object Reference") (OtherActor :type "Actor Object Reference") (OtherComp :type "PrimitiveComponent Object Reference") (OtherBodyIndex :type Integer) (bFromSweep :type Boolean) (SweepResult :type "HitResult Structure (by ref)"))
  (cast `/Game/Casey_Stuff/BP_Player_Pawn` OtherActor)
  (`/Game/Casey_Stuff/BP_PunkdController.PUNKing` (`self.MainController`)))

(fn `UserConstructionScript`)