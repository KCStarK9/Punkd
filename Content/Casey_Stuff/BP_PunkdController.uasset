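; BP_PunkdController is the player controller that moves the BP_Player_Pawn every tick and handles its three-way path choices and "punked" state.
; CHOOSE broadcasts CHOOSING, shows the Choose widget and arms input: forward, left or right teleports the pawn onward, clears widgets, re-possesses it and broadcasts CHOICEMADE.
; PUNKing triggers the pawn's PUNKD, shows that widget and the cursor.
; Look-behind input toggles the pawn's view while held.
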(event `PUNKing`
  (`/Game/Casey_Stuff/BP_Player_Pawn.PUNKD` (`self.Player Pawn`))
  (bind _returnvalue (`|CreateWidget` "/Game/Josh/PUNKD.PUNKD_C"))
  (`UserWidget.AddToViewport` _returnvalue 0)
  (set `self.bShowMouseCursor` true))

(event `self.ReceiveTick`
  (params (DeltaSeconds :type "Float (single-precision)"))
  (`/Game/Casey_Stuff/BP_Player_Pawn.Move` (`self.Player Pawn`)))

(event `EnhancedInput|/Game/Casey_Stuff/Inputs/MoveForward`
  (params (ActionValue :type Boolean) (ElapsedSeconds :type "Float (double-precision)") (TriggeredSeconds :type "Float (double-precision)") (InputAction :type "InputAction Object Reference" :default "/Game/Casey_Stuff/Inputs/MoveForward.MoveForward"))
  (bind _player_pawn (`self.Player Pawn`))
  (:`Triggered`
    (if (`self.MakeaChoice`)
      (`self.K2_SetActorLocation` _player_pawn (+ (`self.K2_GetActorLocation` _player_pawn) (60.0 0.0 0.0)) false true)
      (`WidgetLayoutLibrary.RemoveAllWidgets`)
      (set `self.MakeaChoice` false :!label _label)
      (`self.Possess` (`self.Player Pawn`))
      (`self.CHOICEMADE`))))

(event `EnhancedInput|/Game/Casey_Stuff/Inputs/Right`
  (params (ActionValue :type Boolean) (ElapsedSeconds :type "Float (double-precision)") (TriggeredSeconds :type "Float (double-precision)") (InputAction :type "InputAction Object Reference" :default "/Game/Casey_Stuff/Inputs/Right.Right"))
  (bind _player_pawn (`self.Player Pawn`))
  (:`Triggered`
    (if (`self.MakeaChoice`)
      (`self.K2_SetActorLocation` _player_pawn (+ (`self.K2_GetActorLocation` _player_pawn) (60.0 200.0 0.0)) false true)
      (`WidgetLayoutLibrary.RemoveAllWidgets`)
      (goto _label))))

(event `EnhancedInput|/Game/Casey_Stuff/Inputs/Left`
  (params (ActionValue :type Boolean) (ElapsedSeconds :type "Float (double-precision)") (TriggeredSeconds :type "Float (double-precision)") (InputAction :type "InputAction Object Reference" :default "/Game/Casey_Stuff/Inputs/Left.Left"))
  (bind _player_pawn (`self.Player Pawn`))
  (:`Triggered`
    (if (`self.MakeaChoice`)
      (`self.K2_SetActorLocation` _player_pawn (+ (`self.K2_GetActorLocation` _player_pawn) (60.0 -200.0 0.0)) false true)
      (`WidgetLayoutLibrary.RemoveAllWidgets`)
      (goto _label))))

(event `CHOOSE`
  (`self.CHOOSING`)
  (`UserWidget.AddToViewport` (`self.ChooseWidget`) 0)
  (set `self.MakeaChoice` true))

(event `self.ReceiveBeginPlay`
  (bind _returnvalue (`|CreateWidget` "/Game/Josh/Choose.Choose_C"))
  (set `self.ChooseWidget` _returnvalue)
  (`EnhancedInputSubsystemInterface.AddMappingContext` (subsystem `EnhancedInputLocalPlayerSubsystem`) "/Game/Casey_Stuff/Inputs/Controls.Controls" 0 (struct))
  (bind _outactors (`GameplayStatics.GetAllActorsOfClass` "/Game/Casey_Stuff/PUNK/BP_Punk.BP_Punk_C"))
  (set `self.PUNK` (`|GetArrayItem` _outactors)))

(event `self.ReceivePossess`
  (params (PossessedPawn :type "Pawn Object Reference"))
  (bind _asbp_player_pawn (cast `/Game/Casey_Stuff/BP_Player_Pawn` PossessedPawn))
  (set `self.Player Pawn` _asbp_player_pawn))

(event `EnhancedInput|/Game/Casey_Stuff/Inputs/LookBehind`
  (params (ActionValue :type Boolean) (ElapsedSeconds :type "Float (double-precision)") (TriggeredSeconds :type "Float (double-precision)") (InputAction :type "InputAction Object Reference" :default "/Game/Casey_Stuff/Inputs/LookBehind.LookBehind"))
  (bind _player_pawn (`self.Player Pawn`))
  (:`Started`
    (`/Game/Casey_Stuff/BP_Player_Pawn.LookBehind` _player_pawn))
  (:`Completed`
    (`/Game/Casey_Stuff/BP_Player_Pawn.LookAhead` _player_pawn)))

(fn `UserConstructionScript`)