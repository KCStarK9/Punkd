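; BP_Ball1 is an actor that homes in on the player pawn from where it spawns, then destroys itself.
; On BeginPlay a timeline lerps it, with sweep, from its starting location to the player's current location, re-read on every update.
; When the timeline finishes, it calls BADCHOICE on BP_Player_Pawn, waits briefly, calls RUN, then destroys itself.
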(event `self.ReceiveBeginPlay`
  (bind _returnvalue (`GameplayStatics.GetPlayerPawn` 0))
  (bind _output_get (set `self.StartingLocation` (`self.K2_GetActorLocation`)))
  (bind (_direction _newtrack_0) (`Timeline|Timeline`)
    (:`Update`
      (`self.K2_SetActorLocation` (`KismetMathLibrary.VLerp` _output_get (`self.K2_GetActorLocation` _returnvalue) _newtrack_0) true))
    (:`Finished`
      (bind _asbp_player_pawn (cast `/Game/Casey_Stuff/BP_Player_Pawn` _returnvalue))
      (`/Game/Casey_Stuff/BP_Player_Pawn.BADCHOICE` _asbp_player_pawn 0.0)
      (`KismetSystemLibrary.Delay` 1.0)
      (`/Game/Casey_Stuff/BP_Player_Pawn.RUN` _asbp_player_pawn)
      (`self.K2_DestroyActor`))))

(fn `UserConstructionScript`)