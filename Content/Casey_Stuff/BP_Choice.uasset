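; BP_Choice is a trigger actor that starts a choice moment when the player pawn overlaps its box.
; On overlap it plays a Scrotch sound, starts the choice dialogue audio and teleports the pawn to the actor's location.
; It then hands the dialogue audio component to BP_PunkdController through CHOOSE and blends the player's view to itself.
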(event `self.Box.OnComponentBeginOverlap`
  (params (OverlappedComponent :type "PrimitiveComponent Object Reference") (OtherActor :type "Actor Object Reference") (OtherComp :type "PrimitiveComponent Object Reference") (OtherBodyIndex :type Integer) (bFromSweep :type Boolean) (SweepResult :type "HitResult Structure (by ref)"))
  (bind _returnvalue (`GameplayStatics.GetPlayerController` 0))
  (bind _asbp_player_pawn (cast `/Game/Casey_Stuff/BP_Player_Pawn` OtherActor))
  (`GameplayStatics.PlaySound2D` "/Game/Josh/Sounds/Scrotch.Scrotch" 1.0 1.0 0.0 null null)
  (bind _returnvalue_2 (`GameplayStatics.CreateSound2D` (`self.ChoiceDialogue`) 5.0 1.0 0.0 null false false))
  (`AudioComponent.Play` _returnvalue_2 0.0)
  (`self.K2_TeleportTo` :`self` _asbp_player_pawn :`DestLocation` (`self.K2_GetActorLocation`))
  (bind _asbp_punkd_controller (cast `/Game/Casey_Stuff/BP_PunkdController` _returnvalue))
  (`/Game/Casey_Stuff/BP_PunkdController.CHOOSE` _asbp_punkd_controller _returnvalue_2)
  (`PlayerController.SetViewTargetWithBlend` _returnvalue self 2.0 "VTBlend_Linear" 0.0 true))

(event `self.Box.OnComponentEndOverlap`
  (params (OverlappedComponent :type "PrimitiveComponent Object Reference") (OtherActor :type "Actor Object Reference") (OtherComp :type "PrimitiveComponent Object Reference") (OtherBodyIndex :type Integer)))

(fn `UserConstructionScript`)